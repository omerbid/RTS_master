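; Base settlement actor for the RTS that feeds the game state's resources according to who controls it.
; On BeginPlay, with a valid Archetype, it copies the base population and starts a looping five-second timer.
; Each tick of that timer adds the archetype's gold production to Gold if ControlledBy is the first enum value, otherwise it raises Dread by a fixed amount.
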(event `self.ReceiveBeginPlay`
  (bind _archetype (`self.Archetype`)
    (:`then`
      (if true
        (set `self.Population` (`/Game/RTS/Data/Settlements/DA_SettlementArchetype.BasePopulation` _archetype))
        (`KismetSystemLibrary.K2_SetTimer` null "GenerateResources \n" 5.0 true)))
    (:`else`)))

(event `GenerateResources`
  (bind _asbp_rtsgame_state (cast `/Game/RTS/Blueprints/BP_RTSGameState` (`GameplayStatics.GetGameState`)))
  (if (`|EnumEquality` (`self.ControlledBy`) "NewEnumerator0")
    (set `/Game/RTS/Blueprints/BP_RTSGameState.Gold` (+ (`/Game/RTS/Data/Settlements/DA_SettlementArchetype.BaseGoldProduction` (`self.Archetype`)) (`/Game/RTS/Blueprints/BP_RTSGameState.Gold` _asbp_rtsgame_state)) _asbp_rtsgame_state)
    (`KismetSystemLibrary.PrintString` "Archetype → BaseGoldProduction \n")
    (else
      (set `/Game/RTS/Blueprints/BP_RTSGameState.Dread` (+ (`/Game/RTS/Blueprints/BP_RTSGameState.Dread` _asbp_rtsgame_state) 1.0) _asbp_rtsgame_state))))

(fn `UserConstructionScript`)